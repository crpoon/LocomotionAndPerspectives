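; Player character for a 2.5D view, with jumping and axis-driven movement along world X and Y.
; On BeginPlay it detaches the camera root and stores the starting X, then each tick moves that root to the character's Y and Z while X stays fixed.
; The camera uses pawn control rotation only when a head-mounted display is enabled.
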(event EventBeginPlay
  ;[1 1 1] Initialize Camera
  (Variables|/Script/Engine.CameraComponent|SetbUsePawnControlRotation (Variables|Default|GetCamera) (Class|HeadMountedDisplayFunctionLibrary|IsHeadMountedDisplayEnabled))
  (Class|SceneComponent|DetachfromParent (Variables|Default|GetCameraRoot) true true)
  (Variables|Default|SetCameraXLocation (.x (Transformation|GetActorLocation))))

(event EventTick
  (params (DeltaSeconds :type Float%20%28single-precision%29))
  (bind _returnvalue (Transformation|GetActorLocation))
  ;[1 1 1] Adjust Camera on tick to move with character (y and z)
  (Transformation|SetWorldLocation (Variables|Default|GetCameraRoot) (Math|Vector|MakeVector (Variables|Default|GetCameraXLocation) (.y _returnvalue) (.z _returnvalue)) false false))

(event Input|ActionEvents|InputActionJump
  (params (Key :type Key%20Structure :default "AnyKey"))
  ;[1 1 1] Movement
  (:Pressed
    (Character|Jump))
  (:Released
    (Character|StopJumping)))

(event Input|AxisEvents|InputAxisMoveRight
  (params (AxisValue :type Float%20%28single-precision%29))
  ;[1 1 1] Movement
  (Pawn|Input|AddMovementInput "0,1.000000, 0" AxisValue false))

(event Input|AxisEvents|InputAxisMoveForward
  (params (AxisValue :type Float%20%28single-precision%29))
  ;[1 1 1] Movement
  (Pawn|Input|AddMovementInput "1.000000, 0, 0" AxisValue false))

(fn ConstructionScript)