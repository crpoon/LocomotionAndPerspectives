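; BP_VRCamera is a stationary camera actor that adapts its view depending on whether a head-mounted display is enabled.
; It caches its starting transform on BeginPlay.
; Each tick in VR, it passes that transform through TransformWithHMD and applies the resulting location and rotation.
; Without an HMD, it keeps its location and rotates to look at the first player's pawn.
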(event EventBeginPlay
  (Variables|Default|SetInitial%20Transform (Transformation|GetActorTransform)))

(event EventTick
  (params (DeltaSeconds :type Float%20%28single-precision%29))
  ;[1 1 1] Adjust Camera Angle
  (if (Class|HeadMountedDisplayFunctionLibrary|IsHeadMountedDisplayEnabled)
    (bind _newtransform (CallFunction|TransformwithHMD (Variables|Default|GetInitial%20Transform)))
    (Transformation|SetActorLocationAndRotation (.location _newtransform) (.rotation _newtransform))
    (else
      (Transformation|SetActorRotation (Math|Rotator|FindLookatRotation (Transformation|GetActorLocation) (Transformation|GetActorLocation (Game|Player|GetPlayerPawn 0)))))))

(fn ConstructionScript)